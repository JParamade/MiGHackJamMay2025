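; BP_GenericCharacter is a generic character Blueprint that provides basic health and death handling.
; CE_AddHP calls CE_TakeDamage on every change, adds the amount to HP clamped between zero and MaxHP, then prints the result.
; At zero HP it calls CE_Die, which destroys the actor.
; CE_TakeDamage is an empty event, and BeginPlay, Tick and the construction script do nothing.
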(event Custom|CE_AddHP
  (params (AddHP :type Integer))
  ;[0.6156 0.4372 0 0.5] AddHP
  (CallFunction|CETakeDamage)
  (bind _output_get (Variables|Default|SetHP (Math|Integer|Clamp(Integer) (+ AddHP (Variables|Default|GetHP)) 0 (Variables|Default|GetMaxHP))))
  (Development|PrintText (Utilities|Text|ToText(Integer) _output_get))
  (if (<= (Variables|Default|GetHP) 0)
    (CallFunction|CEDie)))

(event Custom|CE_Die
  ;[0.6323 0.2825 0 0.5] Die
  (Actor|DestroyActor))

(event Custom|CE_TakeDamage)

(event EventBeginPlay)

(event Collision|EventActorBeginOverlap
  (params (OtherActor :type Actor%20Object%20Reference)))

(event EventTick
  (params (DeltaSeconds :type Float%20%28single-precision%29)))

(fn ConstructionScript)