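; Enemy spawner actor that periodically spawns random enemy types around itself and sets them chasing.
; A looping timer started on BeginPlay re-rolls random reachable navigation points within a wide radius until one lies beyond a minimum distance from the spawner.
; It spawns a random class from EnemyClasses there, skipping blocked spots, then calls StartChase on the AIC_Enemy controller reached through the spawned actor's Instigator.
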(event Custom|CE_SpawnEnemy
  (Variables|Default|SetSpawnPoint (.RandomLocation (AI|Navigation|GetRandomReachablePointinRadius (Transformation|GetActorLocation) 7e+03 0 0)))
  (while (<= (Math|Vector|Distance(Vector) (Variables|Default|GetSpawnPoint) (Transformation|GetActorLocation)) 2e+03)
    (Variables|Default|SetSpawnPoint (.RandomLocation (AI|Navigation|GetRandomReachablePointinRadius (Transformation|GetActorLocation) 7e+03 0 0))))
  (bind _returnvalue (Game|SpawnActorfromClass (Utilities|Array|Get(acopy) (Variables|Default|GetEnemyClasses) (Math|Random|RandomIntegerinRange 0 (- (Utilities|Array|Length (Variables|Default|GetEnemyClasses)) 1))) (Math|Transform|MakeTransform (Variables|Default|GetSpawnPoint) "0, 0, 0" "1.000000,1.000000,1.000000") "AdjustIfPossibleButDontSpawnIfColliding" "MultiplyWithRoot" 0 0))
  (Utilities|IsValid _returnvalue
    (:Is%20Valid
      (bind _asaic_enemy (Utilities|Casting|CastToAIC_Enemy (Pawn|GetController (Variables|/Script/Engine.Actor|GetInstigator _returnvalue))))
      (Default|StartChase _asaic_enemy))))

(event EventBeginPlay
  (Utilities|Time|SetTimerbyEvent (delegate Custom|CE_SpawnEnemy) (Variables|Default|GetSpawn%20Cooldown) true))

(fn ConstructionScript)