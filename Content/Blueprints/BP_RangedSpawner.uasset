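; BP_RangedSpawner is a spawner actor that periodically adds BP_RangedEnemy instances to the level.
; A looping timer started on BeginPlay picks a random reachable nav point within a large radius of the spawner.
; It re-rolls points too close to the player, with a capped retry count, then spawns there if collision allows and calls RandomRoam on the enemy.
; Chase-start and random-class selection nodes are left unconnected.
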(event Custom|CE_SpawnEnemy
  (bind _returnvalue (Game|Player|GetPlayerPawn 0))
  (Variables|Default|SetspawnPoint (.RandomLocation (AI|Navigation|GetRandomReachablePointinRadius (Transformation|GetActorLocation) 7e+03 0 0)))
  (Utilities|IsValid _returnvalue
    (:Is%20Valid
      (while (and (<= (Math|Vector|Distance(Vector) (Variables|Default|GetspawnPoint) (Transformation|GetActorLocation _returnvalue)) 1e+03) (< (Variables|Default|GetsecurityCount) 5))
        (Variables|Default|SetSpawnPoint (.RandomLocation (AI|Navigation|GetRandomReachablePointinRadius (Transformation|GetActorLocation) 7e+03 0 0)))
        (Math|Integer|IncrementInt (Variables|Default|GetsecurityCount)))
      (Variables|Default|SetsecurityCount 0)
      (bind _returnvalue_2 (Game|SpawnActorfromClass "/Game/Blueprints/Characters/BP_RangedEnemy.BP_RangedEnemy_C" (Math|Transform|MakeTransform (Math|Vector|MakeVector (.x (Variables|Default|GetspawnPoint)) (.y (Variables|Default|GetspawnPoint)) (.z (Variables|Default|GetspawnPoint))) "0, 0, 0" "1.000000,1.000000,1.000000") "AdjustIfPossibleButDontSpawnIfColliding" "MultiplyWithRoot" 0 0))
      (Utilities|IsValid _returnvalue_2
        (:Is%20Valid
          (Default|RandomRoam _returnvalue_2))))))

(event EventBeginPlay
  (Utilities|Time|SetTimerbyEvent (delegate Custom|CE_SpawnEnemy) (Variables|Default|GetspawnCooldown) true))

(event Collision|EventActorBeginOverlap
  (params (OtherActor :type Actor%20Object%20Reference)))

(event EventTick
  (params (DeltaSeconds :type Float%20%28single-precision%29)))

(fn ConstructionScript)